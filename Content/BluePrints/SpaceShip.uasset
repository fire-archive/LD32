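; Player-controlled physics spaceship with a tractor beam that grabs objects and launches them.
; Thrust axes feed one shared AddForce and yaw, pitch and roll add torque, all only on authority.
; Holding FirePlasmaGun shows the beam and opens a Tick gate that line-traces forward and holds the hit component at a set distance.
; Release hides the beam, closes the gate and impulses the last traced component forward.
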(event EventTick
  (params (DeltaSeconds :type Float%20%28single-precision%29))
  (bind _returnvalue (Transformation|GetActorLocation))
  ;[1 1 1] Find the object hit by the Beam
  (Utilities|FlowControl|Sequence
    (:then_0
      (Utilities|FlowControl|Gate true
        (:Exit
          (bind (_outhit _returnvalue_2) (Collision|LineTraceForObjects _returnvalue (+ _returnvalue (* (Transformation|GetActorForwardVector) (Variables|Default|GetBeamRayCastLength))) (Utilities|Array|MakeArray "ObjectTypeQuery7") false 0 "ForOneFrame"))
          (if _returnvalue_2
            ;[1 1 1] Drag the Beam object with the SpaceShip
            (Transformation|SetWorldLocation (.HitComponent (Collision|BreakHitResult _outhit)) (+ (Transformation|GetActorLocation) (* (Transformation|GetActorForwardVector) (Variables|Default|GetBeamTrackedDistance))) false)
            (Utilities|FlowControl|DoOnce false
              (:Completed
                (Development|PrintString "Beam Locked Target")))))))))

(event Input|ActionEvents|InputActionFirePlasmaGun
  (bind _returnvalue (Transformation|GetActorLocation))
  (bind _returnvalue_2 (Transformation|GetActorForwardVector))
  (bind _beam (Variables|Default|GetBeam))
  ;[1 1 1] Create Beam
  (:Pressed
    (Utilities|FlowControl|Sequence
      (:then_0
        (Components|Activation|Activate _beam false)
        (Rendering|SetVisibility _beam true false))
      (:then_1
        ;[1 1 1] Find the object hit by the Beam
        (Utilities|FlowControl|Gate true) ; enters at Open
      )))
  (:Released
    (Utilities|FlowControl|Sequence
      (:then_0
        (Components|Activation|Deactivate _beam)
        (Rendering|SetVisibility _beam false false))
      (:then_1
        (Utilities|FlowControl|Gate true) ; enters at Close
      )
      (:then_2
        ;[1 1 1] Shoot the tracked object
        (Physics|AddImpulse (.HitComponent (Collision|BreakHitResult (stale EventTick _outhit))) (* _returnvalue_2 (Variables|Default|GetBeamShootImpulsePower)) "None" false)
        (Utilities|FlowControl|DoOnce false) ; enters at Reset
      ))))

(event Input|AxisEvents|InputAxisSideThrust
  (params (AxisValue :type Float%20%28single-precision%29))
  ;[1 1 1] Move Spaceship Sideways
  (Networking|SwitchHasAuthority
    (:Authority
      ;[1 1 1] Apply Torque to the Spaceship
      (Physics|AddForce (+ (* (Transformation|GetActorRightVector) (* AxisValue (Variables|Default|GetMaxSideThrust))) (* (Transformation|GetActorForwardVector) (* (stale Input|AxisEvents|InputAxisThrust AxisValue) (Variables|Default|GetMaxThrust))) (* (Transformation|GetActorUpVector) (* (stale Input|AxisEvents|InputAxisUpDownThrust AxisValue) (Variables|Default|GetMaxUpDownThrust)))) "None" false))))

(event Input|AxisEvents|InputAxisUpDownThrust
  (params (AxisValue :type Float%20%28single-precision%29))
  ;[1 1 1] Move Spaceship Up/Down
  (Networking|SwitchHasAuthority
    (:Authority
      ;[1 1 1] Apply Torque to the Spaceship
      (Physics|AddForce (+ (* (Transformation|GetActorRightVector) (* (stale Input|AxisEvents|InputAxisSideThrust AxisValue) (Variables|Default|GetMaxSideThrust))) (* (Transformation|GetActorForwardVector) (* (stale Input|AxisEvents|InputAxisThrust AxisValue) (Variables|Default|GetMaxThrust))) (* (Transformation|GetActorUpVector) (* AxisValue (Variables|Default|GetMaxUpDownThrust)))) "None" false))))

(event Input|AxisEvents|InputAxisThrust
  (params (AxisValue :type Float%20%28single-precision%29))
  ;[1 1 1] Move Spaceship forward
  (Networking|SwitchHasAuthority
    (:Authority
      ;[1 1 1] Apply Torque to the Spaceship
      (Physics|AddForce (+ (* (Transformation|GetActorRightVector) (* (stale Input|AxisEvents|InputAxisSideThrust AxisValue) (Variables|Default|GetMaxSideThrust))) (* (Transformation|GetActorForwardVector) (* AxisValue (Variables|Default|GetMaxThrust))) (* (Transformation|GetActorUpVector) (* (stale Input|AxisEvents|InputAxisUpDownThrust AxisValue) (Variables|Default|GetMaxUpDownThrust)))) "None" false))))

(event Input|AxisEvents|InputAxisYaw
  (params (AxisValue :type Float%20%28single-precision%29))
  ;[1 1 1] Rotate Spaceshipt round Yaw axis
  (Networking|SwitchHasAuthority
    (:Authority
      (Class|PrimitiveComponent|AddTorque (* (Transformation|GetActorUpVector) (* AxisValue (Variables|Default|GetMaxYawThrust))) "None" false))))

(event Input|AxisEvents|InputAxisRoll
  (params (AxisValue :type Float%20%28single-precision%29))
  ;[1 1 1] Rotate the Spaceshipt around the Roll axis
  (Networking|SwitchHasAuthority
    (:Authority
      (Class|PrimitiveComponent|AddTorque (* (Transformation|GetActorForwardVector) (* AxisValue (Variables|Default|GetMaxRollThrust))) "None" false))))

(event Input|AxisEvents|InputAxisPitch
  (params (AxisValue :type Float%20%28single-precision%29))
  ;[1 1 1] Rotate the Spaceship around the Pitch axis
  (Networking|SwitchHasAuthority
    (:Authority
      (Class|PrimitiveComponent|AddTorque (* (Transformation|GetActorRightVector) (* AxisValue (Variables|Default|GetMaxPitchThrust))) "None" false))))

(fn ConstructionScript)